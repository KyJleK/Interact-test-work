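; BP_SphereTraceObject is a component that repeatedly sphere-traces for chosen object types in front of its owning actor.
; On BeginPlay it sets its tick interval from a variable, then each tick traces along the owner's forward vector using configurable distance, radius and debug drawing.
; It broadcasts the result through OnHit every tick without checking whether anything was hit.
; SetNewEnabled switches the tracing on or off by toggling component tick.
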(event `self.ReceiveBeginPlay`
  (`self.SetComponentTickInterval` (`self.Tick Interval`)))

(event `self.ReceiveTick`
  (params (DeltaSeconds :type "Float (single-precision)"))
  (bind _returnvalue (`self.GetOwner`))
  (bind _returnvalue_2 (`Actor.K2_GetActorLocation` _returnvalue))
  (bind _outhit (`KismetSystemLibrary.SphereTraceSingleForObjects` :`Start` _returnvalue_2 :`End` (+ _returnvalue_2 (* (`Actor.GetActorForwardVector` _returnvalue) (`self.Distance`))) :`Radius` (`self.Radius`) :`ObjectTypes` (`self.Object Types`) :`DrawDebugType` (`self.Draw Debug Type`)))
  (`self.OnHit` _outhit))

(fn `SetNewEnabled`
  (params (`New state` :type Boolean))
  (`self.SetComponentTickEnabled` `New state`))