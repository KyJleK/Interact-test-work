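; BP_Pedestal is an interactable pedestal that takes the item held in a character's arm as a key and opens its referenced door.
; Placing the key destroys the held actor, reveals the pedestal's static mesh and blocks further use.
; The interactability check doubles as the prompt, showing a widget-component nameplate and starting a short timer, apparently to hide it again.
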(event `self.ReceiveBeginPlay`
  (bind _asuw_nameplate (cast `/Game/HUD/Widgets/UW_Nameplate` (`WidgetComponent.GetWidget` (`self.WC_TablePlate`))))
  (set `self.UW_Nameplate` _asuw_nameplate))

(event `/Game/Actors/Common/Interfaces/BI_Interactable.StartInteract`
  (params (Character :type "/Game/ThirdPerson/Blueprints/BP_ThirdPersonCharacter Object Reference"))
  (if (not (`self.KeySetted`))
    (`/Game/ThirdPerson/Blueprints/BP_ThirdPersonCharacter.AttachedActorToArm` Character
      (:`then`
        (`self.SetKey` Character)
        (`/Game/Actors/Door/Blueprints/BP_Door.OpenDoor_event` (`self.DoorRef`)))
      (:`else`))))

(event `HideTableplate`
  (`self.SetVisibilityTableplate` false))

(fn `isInteractable`
  (params (Character :type "/Game/ThirdPerson/Blueprints/BP_ThirdPersonCharacter Object Reference"))
  (returns (Interactable :type Boolean))
  (locals (L_Character :type "/Game/ThirdPerson/Blueprints/BP_ThirdPersonCharacter Object Reference"))
  (bind _output_get (set `local.L_Character` Character))
  (`/Game/ThirdPerson/Blueprints/BP_ThirdPersonCharacter.AttachedActorToArm` _output_get
    (:`then`
      (if (`self.KeySetted`)
        (set `local.L_Character` null)
        (return false)
        (else
          (`self.SetVisibilityTableplate` true)
          (set `self.BP_TPCharacter` (`local.L_Character`))
          (bind _returnvalue (`KismetSystemLibrary.K2_SetTimerDelegate` (`|CreateDelegate` :!event `HideTableplate`) 0.6))
          (set `self.Timer` _returnvalue)
          (return true))))
    (:`else`
      (set `local.L_Character` null)
      (return false))))

(fn `SetKey`
  (params (Character :type "/Game/ThirdPerson/Blueprints/BP_ThirdPersonCharacter Object Reference"))
  (`self.K2_DestroyActor` (`/Game/ThirdPerson/Blueprints/BP_ThirdPersonCharacter.AttachedActorToArm` Character))
  (set `self.KeySetted` true)
  (`SceneComponent.SetVisibility` (`self.StaticMesh`) true false)
  (`KismetSystemLibrary.K2_ClearAndInvalidateTimerHandle` (`self.Timer`))
  (`self.SetVisibilityTableplate` false))

(fn `SetVisibilityTableplate`
  (params (NewVisibility :type Boolean))
  (`/Game/Components/WC_TablePlate.SetNewVisibility` (`self.WC_TablePlate`) NewVisibility))

(fn `UserConstructionScript`)